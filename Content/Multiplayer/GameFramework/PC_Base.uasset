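; PC_Base is a multiplayer player controller Blueprint that handles debug-style hotkeys for the player's HUD.
; Both keys cast the current HUD to HUD_Player: key 1 shows the inventory, while key 0 focuses the chat panel's input box and shows the mouse cursor.
; BeginPlay and Tick are empty, and a console command for the ability system debug display is left unconnected.
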(event EventBeginPlay)

(event EventTick
  (params (DeltaSeconds :type Float%20%28single-precision%29)))

(event Input|KeyboardEvents|0
  (params (Key :type Key%20Structure :default "None"))
  (:Pressed
    (bind _ashud_player (Utilities|Casting|CastToHUD_Player (HUD|GetHUD)))
    (Widget|SetKeyboardFocus (Variables|/Script/Multiplayer.MChatPanelWidget|GetInputMessageBox (Variables|/Script/Multiplayer.MPlayerHUD|GetChatPanelWidget _ashud_player)))
    (Variables|Default|SetbShowMouseCursor true)))

(event Input|KeyboardEvents|1
  (params (Key :type Key%20Structure :default "None"))
  (:Pressed
    (bind _ashud_player (Utilities|Casting|CastToHUD_Player (HUD|GetHUD)))
    (Class|MPlayerHUD|ShowInventory _ashud_player true)))

(fn ConstructionScript)